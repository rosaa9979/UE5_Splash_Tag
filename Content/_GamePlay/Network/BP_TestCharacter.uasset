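; BP_TestCharacter is a networked test character that drives a WidgetInteraction component for pointer input on widgets.
; On BeginPlay it deactivates that component unless the character is both locally controlled and has authority, so remote clients' own characters also deactivate it.
; The IA_Shot Enhanced Input action presses and releases the left mouse pointer key through the component.
; Tick casts the game state to MainMapGameState when locally controlled, but does nothing with the result.
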(event Input|EnhancedActionEvents|EnhancedInputActionIA_Shot
  (params (ActionValue :type Boolean) (ElapsedSeconds :type Float%20%28double-precision%29) (TriggeredSeconds :type Float%20%28double-precision%29) (InputAction :type Input%20Action%20Object%20Reference :default "/Game/_GamePlay/Player/Input/IA_Shot.IA_Shot"))
  (bind _widgetinteraction (Variables|Default|GetWidgetInteraction))
  (:Started
    (Class|WidgetInteractionComponent|PressPointerKey _widgetinteraction "LeftMouseButton"))
  (:Completed
    (Class|WidgetInteractionComponent|ReleasePointerKey _widgetinteraction "LeftMouseButton")))

(event EventBeginPlay
  (if (not (and (Pawn|IsLocallyControlled) (Ability|HasAuthority)))
    (Components|Activation|Deactivate (Variables|Default|GetWidgetInteraction))))

(event EventTick
  (params (DeltaSeconds :type Float%20%28single-precision%29))
  (if (Pawn|IsLocallyControlled)
    (Utilities|Casting|CastToMainMapGameState (Game|GetGameState))))

(fn ConstructionScript)